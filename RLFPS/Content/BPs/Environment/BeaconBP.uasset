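; BeaconBP is an interactive world beacon that awards a gun mod once its event is complete.
; Its widget turns toward the player each tick, shows the NewMod class's image and text, and switches pages with collection state.
; Using it adds a constructed mod to GunBP when completed and activated, otherwise plays the HordeMode sound.
; Sphere overlap by GunBP plays a one-time first-discovery sound tracked in SymGM, except on tutorial beacons.
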(event `self.ReceiveBeginPlay`
  (bind (_name _type _image _infotext) (defaults `Object` (`self.newMod`)))
  (bind _asbeacon_main_widget (cast `/Game/Widgets/Beacon/BeaconMainWidget` (`WidgetComponent.GetWidget` (`self.Widget`))))
  (`Image.SetBrushFromTexture` (`/Game/Widgets/Beacon/BeaconMainWidget.Image_61` _asbeacon_main_widget) _image false)
  (`TextBlock.SetText` (`/Game/Widgets/Beacon/BeaconMainWidget.TextBlock_60` _asbeacon_main_widget) (`KismetTextLibrary.Conv_StringToText` _infotext)))

(event `self.ReceiveTick`
  (params (DeltaSeconds :type "Float (single-precision)"))
  (if (`self.debugDraw`)
    (`KismetSystemLibrary.DrawDebugSphere` (`self.K2_GetActorLocation`) (`self.radius`) 9 (struct :`R` 0.061456 :`G` 1.0 :`A` 1.0) 0.0 2.0))
  (bind _returnvalue (`GameplayStatics.GetActorOfClass` "/Game/BPs/Player/FPS_Player.FPS_Player_C"))
  (`SceneComponent.K2_SetWorldRotation` (`self.Widget`) (`KismetMathLibrary.FindLookAtRotation` (`self.K2_GetActorLocation`) (`self.K2_GetActorLocation` _returnvalue)) false false)
  (if (and (not (`self.modCollected`)) (`self.eventComplete`))
    (bind _asbeacon_main_widget (cast `/Game/Widgets/Beacon/BeaconMainWidget` (`WidgetComponent.GetWidget` (`self.Widget`))))
    (bind _widgetswitcher_21 (`/Game/Widgets/Beacon/BeaconMainWidget.WidgetSwitcher_21` _asbeacon_main_widget))
    (if (!= (`WidgetSwitcher.GetActiveWidgetIndex` _widgetswitcher_21) 2)
      (`WidgetSwitcher.SetActiveWidgetIndex` _widgetswitcher_21 2))))

(event `self.RecieveOnUse`
  (if (and (`self.eventComplete`) (`self.activated`))
    (bind _returnvalue (`|GenericCreateObject` (`self.newMod`) self))
    (bind _returnvalue_2 (`GameplayStatics.GetActorOfClass` "/Game/BPs/Player/GunBP.GunBP_C"))
    (`Gun.AddMod` _returnvalue_2 _returnvalue)
    (bind _asbeacon_main_widget (cast `/Game/Widgets/Beacon/BeaconMainWidget` (`WidgetComponent.GetWidget` (`self.Widget`))))
    (`WidgetSwitcher.SetActiveWidgetIndex` (`/Game/Widgets/Beacon/BeaconMainWidget.WidgetSwitcher_21` _asbeacon_main_widget) 0)
    (set `self.modCollected` true)
    (else
      (bind _asbeacon_main_widget_2 (cast `/Game/Widgets/Beacon/BeaconMainWidget` (`WidgetComponent.GetWidget` (`self.Widget`))))
      (`WidgetSwitcher.SetActiveWidgetIndex` (`/Game/Widgets/Beacon/BeaconMainWidget.WidgetSwitcher_21` _asbeacon_main_widget_2) 0)
      (`GameplayStatics.PlaySound2D` "/Game/Audio/FergusonVoiceLines/HordeMode.HordeMode" 1.0 1.0 0.0 null null))))

(event `self.Sphere.OnComponentBeginOverlap`
  (params (OverlappedComponent :type "PrimitiveComponent Object Reference") (OtherActor :type "Actor Object Reference") (OtherComp :type "PrimitiveComponent Object Reference") (OtherBodyIndex :type Integer) (bFromSweep :type Boolean) (SweepResult :type "HitResult Structure (by ref)"))
  (cast `/Game/BPs/Player/GunBP` OtherActor)
  (if (not (`self.isForTutorial`))
    (bind _assym_gm (cast `/Game/BPs/Game_modes/SymGM` (`GameplayStatics.GetGameMode`)))
    (if (not (`SymbioticGameMode.firstBeaconFound` _assym_gm))
      (set `SymbioticGameMode.firstBeaconFound` true _assym_gm)
      (`GameplayStatics.PlaySound2D` "/Game/Audio/FergusonVoiceLines/FirstBeacon.FirstBeacon" 1.0 1.0 0.0 null null))))

(event `self.PlayActivationSound`
  (`GameplayStatics.PlaySound2D` null 1.0 1.0 0.0 null null))

(fn `UserConstructionScript`)