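; BP_Acid is an acid hazard actor that deals damage over time to Grunts and destroys itself 30 seconds after spawning.
; Overlapping its BoxCollider sets the Grunt's AcidDamage and starts a looping timer calling ApplyAcidDamage on that Grunt every Interval.
; One shared Delay of Duration clears only the latest timer handle, so overlapping several Grunts or destroying the acid mid-delay can leave timers running.
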(event `self.ReceiveBeginPlay`
  (`KismetSystemLibrary.Delay` 30.0)
  (`self.K2_DestroyActor`))

(event `self.BoxCollider.OnComponentBeginOverlap`
  (params (OverlappedComponent :type "PrimitiveComponent Object Reference") (OtherActor :type "Actor Object Reference") (OtherComp :type "PrimitiveComponent Object Reference") (OtherBodyIndex :type Integer) (bFromSweep :type Boolean) (SweepResult :type "HitResult Structure (by ref)"))
  (bind _asgrunt (cast `/Game/BPs/Enemy_systems/AI/Grunt` OtherActor))
  (set `/Game/BPs/Enemy_systems/AI/Grunt.AcidDamage` (`self.damage`) _asgrunt)
  (bind _returnvalue (`KismetSystemLibrary.K2_SetTimer` _asgrunt "ApplyAcidDamage" (`self.interval`) true))
  (`KismetSystemLibrary.Delay` (`self.duration`))
  (`KismetSystemLibrary.K2_ClearAndInvalidateTimerHandle` _returnvalue))

(fn `UserConstructionScript`)